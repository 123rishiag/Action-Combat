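; BP_Boss is a boss enemy character that runs the BT_Boss behavior tree through its AI controller from BeginPlay.
; Pawn sensing passes seen pawns to DetectPawn with the player pawn as target, then creates a WBP_Boss health widget on every sighting, with no guard against duplicates.
; Incoming damage reduces health in the Stats component, whose health percentage delegate updates that widget.
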(event OnSeePawn(PawnSensingComp)
  (params (Pawn :type Pawn%20Object%20Reference))
  (Class|BossCharacter|DetectPawn Pawn (Game|Player|GetPlayerPawn 0))
  (bind _returnvalue (UserInterface|CreateWidget "/Game/UI/WBP_Boss.WBP_Boss_C"))
  (bind _output_get (Variables|Default|SetBoss%20Widget _returnvalue))
  (UserInterface|Viewport|AddtoViewport _output_get 0)
  (Default|SetHealth (Variables|Default|GetBoss%20Widget) (Class|StatsComponent|GetStatPercentage (Variables|Default|GetStats) "Health" "MaxHealth")))

(event OnHealthPercentUpdateDelegate(Stats)
  (params (Percentage :type Float%20%28single-precision%29))
  (Default|SetHealth (Variables|Default|GetBoss%20Widget) Percentage))

(event EventBeginPlay
  (AI|RunBehaviorTree (AI|GetAIController self) "/Game/Characters/AI/BT_Boss.BT_Boss"))

(event Game|Damage|EventAnyDamage
  (params (Damage :type Float%20%28single-precision%29) (DamageType :type Damage%20Type%20Object%20Reference) (InstigatedBy :type Controller%20Object%20Reference) (DamageCauser :type Actor%20Object%20Reference))
  (Class|StatsComponent|ReduceHealth (Variables|Default|GetStats) Damage))

(fn ConstructionScript)